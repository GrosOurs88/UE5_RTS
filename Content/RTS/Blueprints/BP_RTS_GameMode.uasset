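; RTS game mode that gives each joining player control of an RTS camera already in the level.
; On PostLogin it searches all BP_RTS_Camera actors and has the new controller possess the first whose PlayerIndex matches the game mode's counter.
; It then prints the player number on screen and increments the counter for the next login.
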(event EventPostLogin
  (params (NewPlayer :type Player%20Controller%20Object%20Reference))
  (bind _outactors (Actor|GetAllActorsOfClass "/Game/RTS/Blueprints/BP_RTS_Camera.BP_RTS_Camera_C"))
  (bind _array_element (Utilities|Array|ForEachLoopwithBreak _outactors :!label _label)
    (:LoopBody
      (if (== (Variables|/Game/RTS/Blueprints/BP_RTS_Camera.BP_RTS_Camera_C|GetPlayerIndex _array_element) (Variables|Default|GetPlayerIndex))
        (Pawn|Possess NewPlayer _array_element)
        (goto _label Break)))
    (:Completed
      (Development|PrintString (Utilities|String|Append "Player: " (Utilities|String|ToString(Integer) (Variables|Default|GetPlayerIndex))) true true "(R=0.000000,G=0.660000,B=1.000000,A=1.000000)" 1e+01)
      (Math|Integer|IncrementInt (Variables|Default|GetPlayerIndex)))))

(fn ConstructionScript)