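; RTS camera pawn that pans, rotates and zooms through Enhanced Input, adding the IMC_RTS mapping context on BeginPlay.
; Movement input follows the actor's right and forward vectors, rotation applies local yaw, and zoom sets a clamped spring arm length.
; Tick calls MoveCameraToViewport, but its screen-edge scrolling logic is disconnected and never runs.
; Follow, MoveTo and the cursor and finger location queries are empty stubs.
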(event Input|EnhancedActionEvents|EnhancedInputActionINP_RotateCamera
  (params (ActionValue :type Float%20%28double-precision%29) (ElapsedSeconds :type Float%20%28double-precision%29) (TriggeredSeconds :type Float%20%28double-precision%29) (InputAction :type Input%20Action%20Object%20Reference :default "/Game/RTS/Inputs/INP_RotateCamera.INP_RotateCamera"))
  ;[0.1979 0.1979 0.1979] Camera rotation
  (:Triggered
    (Transformation|AddActorLocalRotation (Math|Rotator|MakeRotator 0.0 0.0 (* ActionValue (Variables|Default|GetCameraRotationSpeedMultiplier))) false false)))

(event Input|EnhancedActionEvents|EnhancedInputActionINP_ZoomCamera
  (params (ActionValue :type Float%20%28double-precision%29) (ElapsedSeconds :type Float%20%28double-precision%29) (TriggeredSeconds :type Float%20%28double-precision%29) (InputAction :type Input%20Action%20Object%20Reference :default "/Game/RTS/Inputs/INP_ZoomCamera.INP_ZoomCamera"))
  ;[0.1979 0.1979 0.1979] Camera zoom
  (:Triggered
    (bind _output_get (Variables|Default|SetTargetArmLength (Math|Float|Clamp(Float) (+ (Variables|Default|GetTargetArmLength) (* ActionValue (Variables|Default|GetCameraZoomMultiplier))) (Variables|Default|GetMinZoom) (Variables|Default|GetMaxZoom))))
    (Variables|/Script/Engine.SpringArmComponent|SetTargetArmLength (Variables|Default|GetSpringArm) _output_get)))

(event Input|EnhancedActionEvents|EnhancedInputActionINP_MoveCamera
  (params (ActionValue :type Vector%202D%20Structure) (ElapsedSeconds :type Float%20%28double-precision%29) (TriggeredSeconds :type Float%20%28double-precision%29) (InputAction :type Input%20Action%20Object%20Reference :default "/Game/RTS/Inputs/INP_MoveCamera.INP_MoveCamera"))
  ;[0.1979 0.1979 0.1979] Camera translation
  (:Triggered
    (Pawn|Input|AddMovementInput (* (.x ActionValue) (Transformation|GetActorRightVector)) 1.0 false)
    (Pawn|Input|AddMovementInput (* (.y ActionValue) (Transformation|GetActorForwardVector)) 1.0 false)))

(event EventBeginPlay
  ;[0.1979 0.1979 0.1979] Get Input Mapping Context
  (Input|AddMappingContext (PlayerController|LocalPlayerSubsystems|GetEnhancedInputLocalPlayerSubsystem (Game|GetPlayerController 0)) "/Game/RTS/Inputs/IMC_RTS.IMC_RTS" 0 "(bIgnoreAllPressedKeysUntilRelease=True,bForceImmediately=False)"))

(event Collision|EventActorBeginOverlap
  (params (OtherActor :type Actor%20Object%20Reference)))

(event EventTick
  (params (DeltaSeconds :type Float%20%28single-precision%29))
  (CallFunction|MoveCameratoViewport) ; Check mouse pointer position to move camera
)

(fn ConstructionScript)

(fn MoveCameratoViewport
  ;[0.1979 0.1979 0.1979] Check mouse pointer position to move camera
)

(fn Follow
  (params (Location :type Vector)))

(fn Moveto
  (params (Location :type Vector)))

(fn GetLocationUnderCursor
  (return false "0, 0, 0"))

(fn GetLocationUnderFinger
  (return false "0, 0, 0"))