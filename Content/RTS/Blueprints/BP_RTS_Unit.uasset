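; BP_RTS_Unit is a selectable RTS unit with a team that moves to given destinations through AIMoveTo.
; Releasing a click on it registers it with player controller 0 after a short delay and shows its selection marker.
; Cursor-over events send hover and clear-hover messages to that controller.
; It also exposes selection toggling, a team getter and an always-true interactable check.
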(event Custom|HoverBegin
  (params (TouchedActor :type Actor%20Object%20Reference))
  (Class|BPIPlayerController|OnHover(Message) (Game|GetPlayerController 0)))

(event Custom|EndHover
  (params (TouchedActor :type Actor%20Object%20Reference))
  (Class|BPIPlayerController|ClearHover(Message) (Game|GetPlayerController 0)))

(event EventActorOnReleased
  (params (ButtonReleased :type Key%20Structure :default "None"))
  (Utilities|FlowControl|Delay 0.1)
  (Class|BPIPlayerController|RegisterActor(Message) (Game|GetPlayerController 0) self)
  (CallFunction|ToggleSelect true))

(event MouseInput|EventActorOnClicked
  (params (ButtonPressed :type Key%20Structure :default "None")))

(event EventGoto
  (params (Destination :type Vector :default "0, 0, 0") (Acceptance%20Radius :type Float%20%28double-precision%29))
  (AI|AIMoveTo self Destination 0 Acceptance%20Radius false))

(event EventToggleSelect
  (params (Select/Deselect :type Boolean))
  (Development|SetHiddeninGame (Variables|Default|GetSelectionMarker) (not Select/Deselect) false))

(event EventBeginPlay
  (EventDispatchers|BindEventtoOnBeginCursorOver (delegate Custom|HoverBegin))
  (EventDispatchers|BindEventtoOnEndCursorOver (delegate Custom|EndHover)))

(fn ConstructionScript)

(fn GetTeam
  (return (Variables|Default|GetTeam)))

(fn IsInteractable
  (return true))